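; Player character Blueprint that handles movement input and a dash.
; On BeginPlay it copies HP and move speed from BP_PlayerController, applying the speed to CharacterMovement.
; Forward and right axis inputs drive movement relative to control rotation.
; The SideStep action launches the character along actor forward, then slightly along the control rotation's up vector, with a DoOnce and delay acting as a cooldown.
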(event EventBeginPlay
  (bind _output_get (Variables|Default|SetPCref (.AsBP%20Player%20Controller (Utilities|Casting|CastToBP_PlayerController (Game|GetPlayerController 0)))))
  (bind _playerhp (Default|GetPlayerHP _output_get))
  (Variables|Default|SetPlayerHP _playerhp)
  (bind _playermovespeed (Default|GetPlayerMoveSpeed _output_get))
  (Variables|/Script/Engine.CharacterMovementComponent|SetMaxWalkSpeed (Variables|Character|GetCharacterMovement) _playermovespeed))

(event Collision|EventActorBeginOverlap
  (params (OtherActor :type Actor%20Object%20Reference)))

(event EventTick
  (params (DeltaSeconds :type Float%20%28single-precision%29)))

(event Input|ActionEvents|InputActionSideStep
  (params (Key :type Key%20Structure :default "None"))
  ;[1 1 1] Dash
  (:Pressed
    (Utilities|FlowControl|DoOnce false :!label _label
      (:Completed
        (Character|LaunchCharacter (* (Transformation|GetActorForwardVector) 1.2e+03) false false)
        (Utilities|FlowControl|Delay 0.01)
        (Character|LaunchCharacter (* (Math|Vector|GetUpVector (Pawn|GetControlRotation :!class /Script/Engine.Pawn)) 2e+02) false false)
        (Utilities|FlowControl|Delay 1.0)
        (goto _label Reset)))))

(event Input|AxisEvents|InputAxisMoveForward
  (params (AxisValue :type Float%20%28single-precision%29))
  ;[1 1 1] Move Forward / Backward
  (if (!= AxisValue 0.0)
    (Pawn|Input|AddMovementInput (Math|Vector|GetForwardVector (Math|Rotator|MakeRotator 0.0 0.0 (.yaw (Pawn|GetControlRotation :!class /Script/Engine.Pawn)))) AxisValue false) ; Move Backwards
  ))

(event Input|AxisEvents|InputAxisMoveRight
  (params (AxisValue :type Float%20%28single-precision%29))
  (bind _returnvalue (Pawn|GetControlRotation :!class /Script/Engine.Pawn))
  ;[1 1 1] Move Right / Left
  (if (!= AxisValue 0.0)
    (Pawn|Input|AddMovementInput (Math|Vector|GetRightVector (Math|Rotator|MakeRotator (.roll _returnvalue) 0.0 (.yaw _returnvalue))) AxisValue false) ; Move Right/Left
  ))

(fn ConstructionScript)