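; BP_Sword is a melee weapon that damages what its blade hits, excluding BP_PlayerCharacter actors.
; TriggerSword starts a fast looping timer that line-traces on the Visibility channel between the sword mesh's start and end sockets, until StopTriggerSword clears it.
; Each trace applies fixed damage with no record of previous hits, so one swing can damage the same actor repeatedly.
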(event Custom|TriggerSword
  (bind _returnvalue (Utilities|Time|SetTimerbyEvent (delegate Custom|SwordLineTrace) 0.01 true))
  (Variables|Default|SetTriggerSwordEvent _returnvalue))

(event Custom|SwordLineTrace
  (bind _sword (Variables|Default|GetSword))
  (bind _outhit (Collision|LineTraceByChannel (Transformation|GetSocketLocation _sword "start") (Transformation|GetSocketLocation _sword "end") "TraceTypeQuery1" false 0 "None"))
  (Utilities|Casting|CastToBP_PlayerCharacter (.HitActor (Collision|BreakHitResult _outhit))
    (:CastFailed
      (Game|Damage|ApplyDamage (.HitActor (Collision|BreakHitResult _outhit)) 5e+01 0 0))))

(event Custom|StopTriggerSword
  (Utilities|Time|ClearandInvalidateTimerbyHandle (Variables|Default|GetTriggerSwordEvent)))

(event EventBeginPlay)

(event Collision|EventActorBeginOverlap
  (params (OtherActor :type Actor%20Object%20Reference)))

(event EventTick
  (params (DeltaSeconds :type Float%20%28single-precision%29)))

(fn ConstructionScript)