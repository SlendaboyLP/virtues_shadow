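; Character stat system that holds health and stamina, with functions to get, set, add and reduce current and maximum values.
; A looping timer regenerates stamina by an amount inversely proportional to current stamina, so low stamina refills faster.
; StartHealing runs a heal-over-time timer for a fixed window.
; Reduce functions report death or whether stamina remains, and bar getters divide by a fixed 100 rather than the maximum.
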(event Custom|HealOverTimeEvent
  (Health|AddCurrentHealth (/ (stale Custom|StartHealing HealAmount) (/ (Variables|Default|GetHealDuration) (Variables|Default|GetHealTickTime)))))

(event Custom|RegenStamina
  ;[1 1 1] Stamina Regen Event, Stamina regnerates faster when low Stamina
  (Stamina|AddCurrentStamina (/ (Variables|Stamina|GetStaminaRegenMax) (Math|Float|Clamp(Float) (Variables|Stamina|GetStamina) (Variables|Stamina|GetStaminaRegenMax) (Variables|Stamina|GetMaxStamina)))))

(event Custom|StartHealing
  (params (HealAmount :type Float%20%28double-precision%29))
  (bind _returnvalue (Utilities|Time|SetTimerbyEvent (delegate Custom|HealOverTimeEvent) 0.5 true))
  (Utilities|FlowControl|Delay 4.0)
  (Utilities|Time|ClearandInvalidateTimerbyHandle _returnvalue))

(event EventBeginPlay
  (bind _returnvalue (Utilities|Time|SetTimerbyEvent (delegate Custom|RegenStamina) (Variables|Stamina|GetTickTime) true))
  (Variables|Stamina|SetStaminaRegenTimer _returnvalue))

(event EventTick
  (params (DeltaSeconds :type Float%20%28single-precision%29)))

(fn GetCurrentHealth
  (return (Variables|Health|GetHealth)))

(fn SetCurrentHealth
  (params (NewHealth :type Float%20%28double-precision%29))
  (bind _output_get (Variables|Health|SetHealth (Math|Float|Clamp(Float) NewHealth 0.0 (Variables|Health|GetMaxHealth))))
  (return _output_get))

(fn AddCurrentHealth
  (params (HeathToAdd :type Float%20%28double-precision%29))
  (bind _output_get (Variables|Health|SetHealth (Math|Float|Clamp(Float) (+ (Variables|Health|GetHealth) HeathToAdd) 0.0 (Variables|Health|GetMaxHealth))))
  (return _output_get))

(fn ReduceCurrentHealth
  (params (ReduceHealthBy :type Float%20%28double-precision%29))
  (bind _output_get (Variables|Health|SetHealth (- (Variables|Health|GetHealth) ReduceHealthBy)))
  (return (<= (- (Variables|Health|GetHealth) ReduceHealthBy) 0.0) _output_get))

(fn SetMaxHealth
  (params (NewMaxHealth :type Float%20%28double-precision%29))
  (bind _output_get (Variables|Health|SetMaxHealth NewMaxHealth))
  (return _output_get))

(fn AddMaxHealth
  (params (IncreaseMaxHealthBy :type Float%20%28double-precision%29))
  (bind _output_get (Variables|Health|SetMaxHealth (+ (Variables|Health|GetMaxHealth) IncreaseMaxHealthBy)))
  (return _output_get))

(fn ReduceMaxHealth
  (params (ReduceMaxHealthBy :type Float%20%28double-precision%29))
  (bind _output_get (Variables|Health|SetMaxHealth (- (Variables|Health|GetMaxHealth) ReduceMaxHealthBy)))
  (return _output_get))

(fn GetCurrentHealthBarValue
  (return (/ (Variables|Health|GetHealth) 1e+02)))

(fn GetMaxHealthBarValue
  (return (/ (Variables|Health|GetMaxHealth) 1e+02)))

(fn IsDead
  (return (<= (Variables|Health|GetHealth) 0.0)))

(fn GetCurrentStamina
  (return (Variables|Stamina|GetStamina)))

(fn SetCurrentStamina
  (params (NewStamina :type Float%20%28double-precision%29))
  (bind _output_get (Variables|Stamina|SetStamina (Math|Float|Clamp(Float) NewStamina 0.0 (Variables|Stamina|GetMaxStamina))))
  (return _output_get))

(fn AddCurrentStamina
  (params (StaminaToAdd :type Float%20%28double-precision%29))
  (bind _output_get (Variables|Stamina|SetStamina (Math|Float|Clamp(Float) (+ StaminaToAdd (Variables|Stamina|GetStamina)) 0.0 (Variables|Stamina|GetMaxStamina))))
  (return _output_get))

(fn SetMaxStamina
  (params (NewMaxStamina :type Float%20%28double-precision%29))
  (bind _output_get (Variables|Stamina|SetMaxStamina NewMaxStamina))
  (return _output_get))

(fn GetMaxStamina
  (return (Variables|Stamina|GetMaxStamina)))

(fn ReduceCurrentStamina
  (params (ReduceStaminaBy :type Float%20%28double-precision%29))
  (bind _output_get (Variables|Stamina|SetStamina (Math|Float|Clamp(Float) (- (Variables|Stamina|GetStamina) ReduceStaminaBy) 0.0 (Variables|Stamina|GetMaxStamina))))
  (return _output_get (not (<= (- (Variables|Stamina|GetStamina) ReduceStaminaBy) 0.0))))

(fn AddMaxStamina
  (params (MaxStaminaToAdd :type Float%20%28double-precision%29))
  (bind _output_get (Variables|Stamina|SetMaxStamina (+ MaxStaminaToAdd (Variables|Stamina|GetMaxStamina))))
  (return _output_get))

(fn ReduceMaxStamina
  (params (ReduceMaxStaminaBy :type Float%20%28double-precision%29))
  (bind _output_get (Variables|Stamina|SetMaxStamina (- (Variables|Stamina|GetMaxStamina) ReduceMaxStaminaBy)))
  (return _output_get))

(fn GetCurrentStaminaBarValue
  (return (/ (Variables|Stamina|GetStamina) 1e+02)))

(fn GetMaxStaminaBarValue
  (return (/ (Variables|Stamina|GetMaxStamina) 1e+02)))

(fn GetMaxHealth
  (return (Variables|Health|GetMaxHealth)))