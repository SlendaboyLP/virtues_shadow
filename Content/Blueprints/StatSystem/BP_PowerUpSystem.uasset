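; Power-up system that holds the set of power-ups acquired in the game, such as FleetFooted, Tank and Bolt.
; AddPowerUp maps an enum value to its class, constructs that object and stores it in the PowerUps array as BPP_PowerUpBase, without checking for duplicates.
; HasPowerUp repeats the enum-to-class mapping to return the first instance of that exact class, while GetAllPowerUps exposes the whole array.
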(event EventBeginPlay)

(event EventTick
  (params (DeltaSeconds :type Float%20%28single-precision%29)))

(fn GetAllPowerUps
  (return (Variables|Default|GetPowerUps)))

(fn AddPowerUp
  (params (PowerUp :type PowerUpTypes%20Enum :default "NewEnumerator0"))
  (bind _returnvalue (Game|ConstructObjectfromClass (Utilities|Select :Index PowerUp :NewEnumerator0 "/Game/Blueprints/StatSystem/PowerUps/BPP_FleetFooted.BPP_FleetFooted_C" :NewEnumerator1 "/Game/Blueprints/StatSystem/PowerUps/BPP_Carnivore.BPP_Carnivore_C" :NewEnumerator2 "/Game/Blueprints/StatSystem/PowerUps/BPP_WellFed.BPP_WellFed_C" :NewEnumerator3 "/Game/Blueprints/StatSystem/PowerUps/BPP_SerratedEdge.BPP_SerratedEdge_C" :NewEnumerator4 "/Game/Blueprints/StatSystem/PowerUps/BPP_Tank.BPP_Tank_C" :NewEnumerator5 "/Game/Blueprints/StatSystem/PowerUps/BPP_PowerStance.BPP_PowerStance_C" :NewEnumerator6 "/Game/Blueprints/StatSystem/PowerUps/BPP_HeavyHitter.BPP_HeavyHitter_C" :NewEnumerator7 "/Game/Blueprints/StatSystem/PowerUps/BPP_OnTheEdge.BPP_OnTheEdge_C" :NewEnumerator8 "/Game/Blueprints/StatSystem/PowerUps/BPP_NastyCritter.BPP_NastyCritter_C" :NewEnumerator10 "/Game/Blueprints/StatSystem/PowerUps/BPP_Bolt.BPP_Bolt_C")))
  (bind _asbpp_power_up_base (Utilities|Casting|CastToBPP_PowerUpBase _returnvalue))
  (Utilities|Array|Add (Variables|Default|GetPowerUps) _asbpp_power_up_base))

(fn HasPowerUp
  (params (PowerUp :type PowerUpTypes%20Enum :default "NewEnumerator0"))
  (for _array_element (Variables|Default|GetPowerUps)
    (if (== (Utilities|GetClass _array_element) (Utilities|Select :Index PowerUp :NewEnumerator0 "/Game/Blueprints/StatSystem/PowerUps/BPP_FleetFooted.BPP_FleetFooted_C" :NewEnumerator1 "/Game/Blueprints/StatSystem/PowerUps/BPP_Carnivore.BPP_Carnivore_C" :NewEnumerator2 "/Game/Blueprints/StatSystem/PowerUps/BPP_WellFed.BPP_WellFed_C" :NewEnumerator3 "/Game/Blueprints/StatSystem/PowerUps/BPP_SerratedEdge.BPP_SerratedEdge_C" :NewEnumerator4 "/Game/Blueprints/StatSystem/PowerUps/BPP_Tank.BPP_Tank_C" :NewEnumerator5 "/Game/Blueprints/StatSystem/PowerUps/BPP_PowerStance.BPP_PowerStance_C" :NewEnumerator6 "/Game/Blueprints/StatSystem/PowerUps/BPP_HeavyHitter.BPP_HeavyHitter_C" :NewEnumerator7 "/Game/Blueprints/StatSystem/PowerUps/BPP_OnTheEdge.BPP_OnTheEdge_C" :NewEnumerator8 "/Game/Blueprints/StatSystem/PowerUps/BPP_NastyCritter.BPP_NastyCritter_C" :NewEnumerator10 "/Game/Blueprints/StatSystem/PowerUps/BPP_Bolt.BPP_Bolt_C"))
      (return _array_element (== (Utilities|GetClass _array_element) (Utilities|Select :Index PowerUp :NewEnumerator0 "/Game/Blueprints/StatSystem/PowerUps/BPP_FleetFooted.BPP_FleetFooted_C" :NewEnumerator1 "/Game/Blueprints/StatSystem/PowerUps/BPP_Carnivore.BPP_Carnivore_C" :NewEnumerator2 "/Game/Blueprints/StatSystem/PowerUps/BPP_WellFed.BPP_WellFed_C" :NewEnumerator3 "/Game/Blueprints/StatSystem/PowerUps/BPP_SerratedEdge.BPP_SerratedEdge_C" :NewEnumerator4 "/Game/Blueprints/StatSystem/PowerUps/BPP_Tank.BPP_Tank_C" :NewEnumerator5 "/Game/Blueprints/StatSystem/PowerUps/BPP_PowerStance.BPP_PowerStance_C" :NewEnumerator6 "/Game/Blueprints/StatSystem/PowerUps/BPP_HeavyHitter.BPP_HeavyHitter_C" :NewEnumerator7 "/Game/Blueprints/StatSystem/PowerUps/BPP_OnTheEdge.BPP_OnTheEdge_C" :NewEnumerator8 "/Game/Blueprints/StatSystem/PowerUps/BPP_NastyCritter.BPP_NastyCritter_C" :NewEnumerator10 "/Game/Blueprints/StatSystem/PowerUps/BPP_Bolt.BPP_Bolt_C"))))))