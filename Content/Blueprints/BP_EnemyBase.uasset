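; Base enemy character Blueprint that chases the player and dies when its health runs out.
; PawnSensing spots the player character and issues an AI MoveTo toward it, with walk speed set on BeginPlay.
; Any damage lowers an integer Health, prints it to screen, and destroys the enemy after a short delay once it reaches zero.
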(event OnSeePawn(PawnSensing)
  (params (Pawn :type Pawn%20Object%20Reference))
  (bind _asbp_player_character (Utilities|Casting|CastToBP_PlayerCharacter Pawn))
  (AI|AIMoveTo self "0, 0, 0" _asbp_player_character 5e+01 true))

(event EventBeginPlay
  (Variables|/Script/Engine.CharacterMovementComponent|SetMaxWalkSpeed (Variables|Character|GetCharacterMovement) 5e+02))

(event Collision|EventActorBeginOverlap
  (params (OtherActor :type Actor%20Object%20Reference)))

(event EventTick
  (params (DeltaSeconds :type Float%20%28single-precision%29)))

(event Game|Damage|EventAnyDamage
  (params (Damage :type Float%20%28single-precision%29) (DamageType :type Damage%20Type%20Object%20Reference) (InstigatedBy :type Controller%20Object%20Reference) (DamageCauser :type Actor%20Object%20Reference))
  (bind _output_get (Variables|Default|SetHealth (Math|Conversions|ToInteger(Byte) (- (Variables|Default|GetHealth) (Class|KismetMathLibrary|ToInt64(Float) Damage)))))
  (Development|PrintString (Utilities|String|ToString(Integer) _output_get))
  (if (<= _output_get 0)
    (Utilities|FlowControl|Delay 1.0)
    (Actor|DestroyActor)))

(fn ConstructionScript)