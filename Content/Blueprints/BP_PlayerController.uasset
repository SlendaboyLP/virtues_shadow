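; BP_PlayerController is a player controller Blueprint that stores player state: a sphere counter, move speed and HP.
; Each value is exposed through a simple getter and setter function, with no clamping, validation or change notification.
; The event graph and construction script contain no active logic, so the asset acts purely as a data holder.
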(event EventBeginPlay)

(event EventTick
  (params (DeltaSeconds :type Float%20%28single-precision%29)))

(fn ConstructionScript)

(fn GetSphereCount
  (return (Variables|Default|GetSphereCounter)))

(fn SetSphereCount
  (params (SphereCount :type Integer))
  (Variables|Default|SetSphereCounter SphereCount))

(fn GetPlayerMoveSpeed
  (return (Variables|Default|GetPlayerMoveSpeed)))

(fn SetPlayerMoveSpeed
  (params (PlayerMoveSpeed :type Float%20%28double-precision%29))
  (Variables|Default|SetPlayerMoveSpeed PlayerMoveSpeed))

(fn GetPlayerHP
  (return (Variables|Default|GetPlayerHP)))

(fn SetPlayerHP
  (params (PlayerHP :type Integer))
  (Variables|Default|SetPlayerHP PlayerHP))