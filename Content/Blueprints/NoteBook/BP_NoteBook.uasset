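; BP_NoteBook is an interactable notebook actor that shows and hides an on-screen note.
; Shortly after BeginPlay it creates a WB_NoteBook widget and fills it with the actor's NoteBookText.
; Interact toggles that cached widget on and off the viewport, tracking the state with IsOpen.
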(event EventBeginPlay
  (Utilities|FlowControl|Delay 0.2)
  (bind _returnvalue (UserInterface|CreateWidget "/Game/Widgets/WB_NoteBook.WB_NoteBook_C"))
  (bind _output_get (Variables|Default|SetNoteBookWidget _returnvalue))
  (Default|SetNoteBookText _output_get (Variables|Default|GetNoteBookText)))

(event Collision|EventActorBeginOverlap
  (params (OtherActor :type Actor%20Object%20Reference)))

(event EventTick
  (params (DeltaSeconds :type Float%20%28single-precision%29)))

(event EventInteract
  (bind _notebookwidget (Variables|Default|GetNoteBookWidget))
  (if (Variables|Default|GetIsOpen)
    (Widget|RemovefromParent _notebookwidget)
    (Variables|Default|SetIsOpen false)
    (else
      (UserInterface|Viewport|AddtoViewport _notebookwidget 0)
      (Variables|Default|SetIsOpen true))))

(fn ConstructionScript)