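; Base enemy character with health, an overhead health widget, and contact damage to the player.
; Overlapping the player starts a looping timer that applies damage each tick until overlap ends.
; Non-DoT hits pass a DoOnce that resets after a hit montage and short delay, while damage-over-time bypasses this gate.
; At zero health it stops AI logic and destroys itself after a delay.
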(event Custom|DealDamage
  ;[1 1 1] Wenn Character in die Nähe des Gegners kommt
  (Game|Damage|ApplyDamage (stale Collision|EventActorBeginOverlap _asbp_player_character) (Variables|Default|GetDamageToPlayerPerTick) 0 0 "/Script/Engine.DamageType"))

(event EventBeginPlay
  (Rendering|SetCastShadow (Variables|Default|GetWidget) false)
  (CallFunction|UpdateHealthBar))

(event Collision|EventActorBeginOverlap
  (params (OtherActor :type Actor%20Object%20Reference))
  ;[1 1 1] Wenn Character in die Nähe des Gegners kommt
  (bind _asbp_player_character (Utilities|Casting|CastToBP_PlayerCharacter OtherActor))
  (bind _returnvalue (Utilities|Time|SetTimerbyEvent (delegate Custom|DealDamage) 0.1 true))
  (Variables|Default|SetDealDamageTimer _returnvalue))

(event EventTick
  (params (DeltaSeconds :type Float%20%28single-precision%29)))

(event Game|Damage|EventAnyDamage
  (params (Damage :type Float%20%28single-precision%29) (DamageType :type Damage%20Type%20Object%20Reference) (InstigatedBy :type Controller%20Object%20Reference) (DamageCauser :type Actor%20Object%20Reference))
  (if (== (Utilities|GetClass DamageType) "/Game/Blueprints/DamageTypes/BP_DamageOverTime.BP_DamageOverTime_C")
    (Variables|Default|SetHealth (- (Variables|Default|GetHealth) Damage))
    (CallFunction|UpdateHealthBar)
    (if (CallFunction|IsDead)
      (Utilities|PlayDeath))
    (else
      (Utilities|FlowControl|DoOnce false :!label _label
        (:Completed
          (if (<= (- (Variables|Default|GetHealth) Damage) 0.0)
            (Variables|Default|SetHealth 0.0)
            (else
              (Variables|Default|SetHealth (- (Variables|Default|GetHealth) Damage))))
          (CallFunction|UpdateHealthBar)
          (if (CallFunction|IsDead)
            (Utilities|PlayDeath)
            (else
              ;[1 1 1] Get Hit Animation Missing
              (Animation|PlayAnimMontage "/Game/Animations/Getting_Hit_Anim_Montage.Getting_Hit_Anim_Montage" 3.0 "None")
              (Utilities|FlowControl|Delay 0.2)
              (goto _label Reset))))))))

(event Collision|EventActorEndOverlap
  (params (OtherActor :type Actor%20Object%20Reference))
  ;[1 1 1] Wenn Character in die Nähe des Gegners kommt
  (Utilities|Casting|CastToBP_PlayerCharacter OtherActor)
  (Utilities|Time|ClearandInvalidateTimerbyHandle (Variables|Default|GetDealDamageTimer)))

(fn ConstructionScript)

(fn UpdateWalkSpeed
  (params (NewWalkSpeed :type Float%20%28double-precision%29))
  (Variables|/Script/Engine.CharacterMovementComponent|SetMaxWalkSpeed (Variables|Character|GetCharacterMovement) NewWalkSpeed))

(fn IsDead
  (return (<= (Variables|Default|GetHealth) 0.0)))

(fn UpdateHealthBar
  (bind _health (Variables|Default|GetHealth))
  (bind _aswb_enemy_health (Utilities|Casting|CastToWB_EnemyHealth (UserInterface|GetWidget (Variables|Default|GetWidget))))
  (Progress|SetPercent (Variables|/Game/Widgets/WB_EnemyHealth.WB_EnemyHealth_C|GetEnemyHealthBar _aswb_enemy_health) (/ _health 1e+02))
  (Rendering|Components|TextRender|SetText (Variables|/Game/Widgets/WB_EnemyHealth.WB_EnemyHealth_C|GetEnemyHealthText _aswb_enemy_health) (Utilities|Text|ToText(String) (Utilities|String|ToString(Float) _health))))